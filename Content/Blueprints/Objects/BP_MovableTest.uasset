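; BP_MovableTest is a test movable object that travels in response to the game character entering and leaving trigger volumes.
; Entering MoveBeginTrigger starts the Move component forward, while leaving MoveEndTrigger reverses it and sets ShouldStop.
; When the returning object reaches the non-end endpoint with that flag set, movement is disabled and reset.
; A separate Collect event plays a camera shutter sound through the Shutter component.
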(event OnComponentBeginOverlap(MoveBeginTrigger)
  (params (OverlappedComponent :type Primitive%20Component%20Object%20Reference) (OtherActor :type Actor%20Object%20Reference) (OtherComp :type Primitive%20Component%20Object%20Reference) (OtherBodyIndex :type Integer) (bFromSweep :type Boolean) (SweepResult :type Hit%20Result%20Structure%20%28by%20ref%29))
  (bind _move (Variables|Default|GetMove))
  (Utilities|Casting|CastToBP_GameCharacter OtherActor)
  (Class|MoveComponent|EnableMovement _move true)
  (Class|MoveComponent|SetMoveDirection _move 1)
  (Variables|Default|SetShouldStop false))

(event OnComponentEndOverlap(MoveEndTrigger)
  (params (OverlappedComponent :type Primitive%20Component%20Object%20Reference) (OtherActor :type Actor%20Object%20Reference) (OtherComp :type Primitive%20Component%20Object%20Reference) (OtherBodyIndex :type Integer))
  (Utilities|Casting|CastToBP_GameCharacter OtherActor)
  (Class|MoveComponent|SetMoveDirection (Variables|Default|GetMove) -1)
  (Variables|Default|SetShouldStop true))

(event OnEndpointReached(Move)
  (params (bIsEndPoint :type Boolean))
  (bind _move (Variables|Default|GetMove))
  (if (and (not bIsEndPoint) (Variables|Default|GetShouldStop))
    (Class|MoveComponent|EnableMovement _move false)
    (Class|MoveComponent|ResetMovement _move)))

(event EventCollect
  (params (SourceObj :type Object%20Object%20Reference) (Count :type Float%20%28single-precision%29))
  (bind _shutter (Variables|Default|GetShutter))
  (Audio|Components|Audio|SetSound _shutter "/Engine/VREditor/Sounds/UI/Camera_Shutter.Camera_Shutter")
  (Audio|Components|Audio|Play _shutter 0.0))

(fn ConstructionScript)